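; TemplatePickup is a pickup actor that shows a text prompt widget when the player character is near.
; On BeginPlay it writes itself into ItemInfo, passes the item and pickup text to its PickupText widget, and caches the player's ThirdPersonCharacter.
; Trigger overlaps with a ThirdPersonCharacter show and hide the widget.
; Both begin and end overlap set IsInRange to true, so the flag is never cleared here.
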(event `self.ReceiveBeginPlay`
  (bind _iteminfo (`self.ItemInfo`))
  (bind _pickup_text_reference (`self.Pickup Text Reference`))
  (bind (_item _itemimage _pickuptext) (break `/Game/Blueprints/InventoryStruct` _iteminfo))
  (bind _aspickup_text (cast `/Game/UMG/PickupText` (`WidgetComponent.GetUserWidgetObject` (`self.Widget`))))
  (set `self.Pickup Text Reference` _aspickup_text)
  (setmembers `/Game/Blueprints/InventoryStruct` :`StructRef` _iteminfo :`Item` self)
  (set `/Game/UMG/PickupText.PickupActor` _item _pickup_text_reference)
  (set `/Game/UMG/PickupText.PickupText` _pickuptext _pickup_text_reference)
  (bind _asthird_person_character (cast `/Game/ThirdPersonCPP/Blueprints/ThirdPersonCharacter` (`GameplayStatics.GetPlayerCharacter` 0)))
  (set `self.CharacterReference` _asthird_person_character))

(event `self.Trigger.OnComponentBeginOverlap`
  (params (OverlappedComponent :type "PrimitiveComponent Object Reference") (OtherActor :type "Actor Object Reference") (OtherComp :type "PrimitiveComponent Object Reference") (OtherBodyIndex :type Integer) (bFromSweep :type Boolean) (SweepResult :type "HitResult Structure (by ref)"))
  (cast `/Game/ThirdPersonCPP/Blueprints/ThirdPersonCharacter` OtherActor)
  (`SceneComponent.SetVisibility` (`self.Widget`) true false)
  (set `self.IsInRange` true))

(event `self.Trigger.OnComponentEndOverlap`
  (params (OverlappedComponent :type "PrimitiveComponent Object Reference") (OtherActor :type "Actor Object Reference") (OtherComp :type "PrimitiveComponent Object Reference") (OtherBodyIndex :type Integer))
  (cast `/Game/ThirdPersonCPP/Blueprints/ThirdPersonCharacter` OtherActor)
  (`SceneComponent.SetVisibility` (`self.Widget`) false false)
  (set `self.IsInRange` true))

(fn `UserConstructionScript`)